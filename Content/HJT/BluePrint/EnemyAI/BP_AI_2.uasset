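; BP_AI_2 is an enemy AI actor that carries a soldier count, shown on a text label turned toward the player camera.
; Tick refreshes that label and calls the soldier regeneration, which uses a two-second Delay before adding Resume.
; GetSupply adds a supply bonus, clamped like regeneration to MaxSoldier.
; The sphere hit event is empty; logic subtracting the player character's soldiers and destroying the actor below zero is disconnected.
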(event `Soldier_Resume`
  ;[1 1 1] 增加
  (`KismetSystemLibrary.Delay` 2.0)
  (set `self.Soldier` (`KismetMathLibrary.FClamp` (+ (`self.Soldier`) (`self.Resume`)) 0.0 (`self.Max_Soldier`))))

(event `self.ReceiveTick`
  (params (DeltaSeconds :type "Float (single-precision)"))
  (`self.Soldier_Resume`)
  (`SceneComponent.K2_SetWorldRotation` (`self.TextRender`) (`KismetMathLibrary.FindLookAtRotation` (`SceneComponent.K2_GetComponentLocation` (`self.TextRender`)) (`PlayerCameraManager.GetCameraLocation` (`GameplayStatics.GetPlayerCameraManager` 0))) false false)
  (`TextRenderComponent.K2_SetText` (`self.TextRender`) (`KismetTextLibrary.Conv_DoubleToText` (`self.Soldier`) "HalfToEven")))

(event `self.AI_Sphere.OnComponentHit`
  (params (HitComponent :type "PrimitiveComponent Object Reference") (OtherActor :type "Actor Object Reference") (OtherComp :type "PrimitiveComponent Object Reference") (NormalImpulse :type "Vector Structure") (Hit :type "HitResult Structure (by ref)")))

(event `GetSupply`
  ;[1 1 1] 吃球
  (set `self.Soldier` (`KismetMathLibrary.FClamp` (+ (`self.Soldier`) (`self.Supply`)) 0.0 (`self.Max_Soldier`))))

(fn `UserConstructionScript`)